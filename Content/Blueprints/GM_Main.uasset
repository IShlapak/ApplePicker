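; GM_Main is the main game mode, providing the score and life rules for the player.
; It caches BP_GameState on BeginPlay and stores score, lives and alive state there.
; AddScore and LoseLife each adjust their counter by one, then refresh the HUD through the first player's BP_PlayerController.
; When lives reach zero, LoseLife calls GameOver on BP_GameInstance, then clears IsAlive.
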(event EventBeginPlay
  (bind _asbp_game_state (Utilities|Casting|CastToBP_GameState (Game|GetGameState)))
  (Variables|Default|SetMyGameState _asbp_game_state))

(event EventTick
  (params (DeltaSeconds :type Float%20%28single-precision%29)))

(fn ConstructionScript)

(fn AddScore
  (bind _result (Math|Integer|IncrementInt (Variables|/Game/Blueprints/BP_GameState.BP_GameState_C|GetPlayerScore (Variables|Default|GetMyGameState)))
    (:%20%20
      (Variables|/Game/Blueprints/BP_GameState.BP_GameState_C|SetPlayerScore (Variables|Default|GetMyGameState) _result)
      (bind _asbp_player_controller (Utilities|Casting|CastToBP_PlayerController (Game|GetPlayerController 0)))
      (Default|Update (Variables|/Game/Blueprints/BP_PlayerController.BP_PlayerController_C|GetHUD _asbp_player_controller)))))

(fn LoseLife
  (bind _result (Math|Integer|DecrementInt (Variables|/Game/Blueprints/BP_GameState.BP_GameState_C|GetPlayerLifes (Variables|Default|GetMyGameState)))
    (:%20%20
      (bind _output_get (Variables|/Game/Blueprints/BP_GameState.BP_GameState_C|SetPlayerLifes (Variables|Default|GetMyGameState) _result))
      (bind _asbp_player_controller (Utilities|Casting|CastToBP_PlayerController (Game|GetPlayerController 0)))
      (Default|Update (Variables|/Game/Blueprints/BP_PlayerController.BP_PlayerController_C|GetHUD _asbp_player_controller))
      (if (== _output_get 0)
        (bind _asbp_game_instance (Utilities|Casting|CastToBP_GameInstance (Game|GetGameInstance)))
        (Default|GameOver _asbp_game_instance)
        (Variables|/Game/Blueprints/BP_GameState.BP_GameState_C|SetIsAlive (Variables|Default|GetMyGameState) false)))))