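; BP_AppleTree is a pawn that slides sideways and drops apples while the player is alive.
; Each Tick, if BP_APGameState reports Alive, it moves along its right vector with sweep and runs two countdown timers.
; One timer randomly reverses Speed by a set chance; the other spawns BP_Apple just below the tree.
; Overlapping a BlockingVolume with its Sphere also reverses direction.
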(event OnComponentBeginOverlap(Sphere)
  (params (OverlappedComponent :type Primitive%20Component%20Object%20Reference) (OtherActor :type Actor%20Object%20Reference) (OtherComp :type Primitive%20Component%20Object%20Reference) (OtherBodyIndex :type Integer) (bFromSweep :type Boolean) (SweepResult :type Hit%20Result%20Structure%20%28by%20ref%29))
  (Utilities|Casting|CastToBlockingVolume OtherActor)
  (Variables|Default|SetSpeed (* (Variables|Default|GetSpeed) -1.0)))

(event EventBeginPlay
  (Variables|Default|SetLeftTimeToChangeDirection (Variables|Default|GetChangeDirectionInterval))
  (Variables|Default|SetLeftTimeToSpawnApple (Variables|Default|GetSpawnAppleInterval)))

(event Collision|EventActorBeginOverlap
  (params (OtherActor :type Actor%20Object%20Reference)))

(event EventTick
  (params (DeltaSeconds :type Float%20%28single-precision%29))
  (bind _newparam (CallFunction|IsPlayerAlive))
  (if _newparam
    (CallFunction|CheckDirection DeltaSeconds)
    (Transformation|AddActorWorldOffset (* (Transformation|GetActorRightVector) (* DeltaSeconds (Variables|Default|GetSpeed))) true)
    (CallFunction|CheckAppleSpawn DeltaSeconds)))

(fn ConstructionScript)

(fn CheckDirection
  (params (DeltaTime :type Float%20%28single-precision%29))
  (Variables|Default|SetLeftTimeToChangeDirection (- (Variables|Default|GetLeftTimeToChangeDirection) DeltaTime))
  (if (< (Variables|Default|GetLeftTimeToChangeDirection) 0.0)
    (if (< (Math|Random|RandomFloat) (Variables|Default|GetChanceOfDirectionChange%20))
      (Variables|Default|SetSpeed (* (Variables|Default|GetSpeed) -1.0)))
    (Variables|Default|SetLeftTimeToChangeDirection (Variables|Default|GetChangeDirectionInterval))))

(fn CheckAppleSpawn
  (params (DeltaTime :type Float%20%28single-precision%29))
  (bind _returnvalue (Transformation|GetActorLocation))
  (Variables|Default|SetLeftTimeToSpawnApple (- (Variables|Default|GetLeftTimeToSpawnApple) DeltaTime))
  (if (< (Variables|Default|GetLeftTimeToSpawnApple) 0.0)
    (Game|SpawnActorfromClass "/Game/Blueprints/Pawns/BP_Apple.BP_Apple_C" (Math|Transform|MakeTransform (Math|Vector|MakeVector (.x _returnvalue) (.y _returnvalue) (- (.z _returnvalue) 1e+02)) "0, 0, 0" "1,1,1") "AlwaysSpawn" 0 0)
    (Variables|Default|SetLeftTimeToSpawnApple (Variables|Default|GetSpawnAppleInterval))))

(fn IsPlayerAlive
  (bind _asbp_apgame_state (Utilities|Casting|CastToBP_APGameState (Game|GetGameState)))
  (return (Variables|/Script/ApplePicker.APGameState|GetAlive _asbp_apgame_state)))