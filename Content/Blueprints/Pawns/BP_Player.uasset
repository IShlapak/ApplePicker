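; BP_Player is the player pawn of an apple-catching game, tracking lives and owning the HUD.
; On BeginPlay in the Main level it creates the HUD and starts a game with three lives and the score displayed.
; Apples hitting the Basket component are destroyed and add score through BP_GameState.
; LoseLife updates the HUD and, at zero, clears IsAlive on the GameState and calls GameOver on the GameInstance.
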(event OnComponentHit(Basket)
  (params (HitComponent :type Primitive%20Component%20Object%20Reference) (OtherActor :type Actor%20Object%20Reference) (OtherComp :type Primitive%20Component%20Object%20Reference) (NormalImpulse :type Vector :default "0, 0, 0") (Hit :type Hit%20Result%20Structure%20%28by%20ref%29))
  (bind _asbp_apple (Utilities|Casting|CastToBP_Apple OtherActor))
  (Actor|DestroyActor _asbp_apple)
  (bind _asbp_game_state (Utilities|Casting|CastToBP_GameState (Game|GetGameState)))
  (Default|AddScore _asbp_game_state))

(event EventBeginPlay
  (bind _returnvalue (Game|GetCurrentLevelName true))
  (if (Utilities|Enum|Equal(Enum) _returnvalue "Main")
    (bind _returnvalue_2 (UserInterface|CreateWidget "/Game/Blueprints/CPP/UI/WBP_PlayerHud.WBP_PlayerHud_C"))
    (UserInterface|Viewport|AddtoViewport _returnvalue_2 0)
    (CallFunction|StartNewGame _returnvalue_2)))

(event Collision|EventActorBeginOverlap
  (params (OtherActor :type Actor%20Object%20Reference)))

(event EventTick
  (params (DeltaSeconds :type Float%20%28single-precision%29)))

(fn ConstructionScript)

(fn StartNewGame
  (params (HUD :type WBP%20Player%20Hud%20Object%20Reference))
  (bind _output_get (Variables|Default|SetPlayerHUD HUD))
  (bind _output_get_2 (Variables|Default|SetLifes 3))
  (Class|PlayerGameHud|SetHP _output_get _output_get_2)
  (bind _asbp_game_state (Utilities|Casting|CastToBP_GameState (Game|GetGameState)))
  (Default|SetScoretoHUD _asbp_game_state))

(fn LoseLife
  (bind _result (Math|Integer|DecrementInt (Variables|Default|GetLifes))
    (:%20%20
      (Class|PlayerGameHud|SetHP (Variables|Default|GetPlayerHUD) _result)
      (if (== _result 0)
        (Utilities|FlowControl|Sequence
          (:then_0
            (bind _asbp_game_state (Utilities|Casting|CastToBP_GameState (Game|GetGameState)))
            (Variables|/Game/Blueprints/BP_GameState.BP_GameState_C|SetIsAlive _asbp_game_state false))
          (:then_1
            (bind _asbp_game_instance (Utilities|Casting|CastToBP_GameInstance (Game|GetGameInstance)))
            (Default|GameOver _asbp_game_instance)))))))