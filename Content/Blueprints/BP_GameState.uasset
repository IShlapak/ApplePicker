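; BP_GameState holds the player's score and an alive flag for the game.
; On BeginPlay in the Main level, it sets the alive flag and zeroes the score.
; AddScore increments the score, then SetScoreToHUD pushes the new value to the HUD widget owned by BP_Player, found by casting the first player pawn.
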(event EventBeginPlay
  (bind _returnvalue (Game|GetCurrentLevelName true))
  (if (Utilities|Enum|Equal(Enum) _returnvalue "Main")
    (Variables|Default|SetIsAlive true)
    (Variables|Default|SetPlayerScore 0)))

(event EventTick
  (params (DeltaSeconds :type Float%20%28single-precision%29)))

(fn ConstructionScript)

(fn AddScore
  (Math|Integer|IncrementInt (Variables|Default|GetPlayerScore)
    (:%20%20
      (CallFunction|SetScoretoHUD))))

(fn SetScoretoHUD
  (bind _asbp_player (Utilities|Casting|CastToBP_Player (Game|Player|GetPlayerPawn 0)))
  (Default|SetScore (Variables|/Game/Blueprints/Pawns/BP_Player.BP_Player_C|GetPlayerHUD _asbp_player) (Variables|Default|GetPlayerScore)))