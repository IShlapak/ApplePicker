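; Player controller that drives the BP_Player pawn's sideways movement and opens the pause screen.
; On BeginPlay it caches the pawn, then the LeftRight axis offsets it along its right vector, scaled by the pawn's MaxSpeed, with sweep.
; The offset is applied per input event without delta-time scaling.
; The Pause action delegates to ShowPause on BP_APGameInstance.
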(event EventBeginPlay
  (bind _asbp_player (Utilities|Casting|CastToBP_Player (Game|Player|GetPlayerPawn 0)))
  (Variables|Default|SetPlayerPawn _asbp_player))

(event Input|ActionEvents|InputActionPause
  (params (Key :type Key%20Structure :default "None"))
  (:Pressed
    (bind _asbp_apgame_instance (Utilities|Casting|CastToBP_APGameInstance (Game|GetGameInstance)))
    (Class|APGameInstance|ShowPause _asbp_apgame_instance)))

(event Input|AxisEvents|InputAxisLeftRight
  (params (AxisValue :type Float%20%28single-precision%29))
  (Transformation|AddActorWorldOffset (Variables|Default|GetPlayerPawn) (* (Transformation|GetActorRightVector (Variables|Default|GetPlayerPawn)) (* AxisValue (Variables|/Game/Blueprints/Pawns/BP_Player.BP_Player_C|GetMaxSpeed (Variables|Default|GetPlayerPawn)))) true))

(fn ConstructionScript)